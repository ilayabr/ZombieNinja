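; Enemy actor for the weapon system that tracks health and reports its death and contact with the player.
; DealDamage subtracts from HP, prints the remaining value, and at zero or below calls EnemyDeath and destroys the actor.
; Overlapping a BP_WeaponController actor calls PlayerOverlap.
; ChaseTick is an empty stub, and CheckTragetDistanceInRange is a placeholder comparing the actor's location to itself, so always false.
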(event `self.ReceiveBeginPlay`
  (set `self.HP` (`self.MaxHP`)))

(event `/Game/WeaponSystem/Interface/Weapons/IDamageable.DealDamage`
  (params (DamageAmount :type Integer))
  (bind _output_get (set `self.HP` (- (`self.HP`) DamageAmount)))
  (if (<= _output_get 0)
    (`self.EnemyDeath`)
    (`self.K2_DestroyActor`)
    (`KismetSystemLibrary.PrintString` (`KismetStringLibrary.Concat_StrStr` "0" " HP") true true (struct :`G` 1.0 :`A` 1.0) 5.0)
    (else
      (`KismetSystemLibrary.PrintString` (`KismetStringLibrary.Concat_StrStr` (`KismetStringLibrary.Conv_IntToString` (`self.HP`)) " HP") true true (struct :`G` 1.0 :`A` 1.0) 5.0))))

(event `self.ReceiveActorBeginOverlap`
  (params (OtherActor :type "Actor Object Reference"))
  (cast `/Game/WeaponSystem/Player/BP_WeaponController` OtherActor)
  (`self.PlayerOverlap`))

(fn `ChaseTick`
  (params (`delta time` :type "Float (double-precision)")))

(fn `CheckTragetDistanceInRange`
  (returns (IsInRange :type Boolean))
  (return (< (`KismetMathLibrary.Vector_Distance` (`self.K2_GetActorLocation`) (`self.K2_GetActorLocation`)) 0.0)))

(fn `UserConstructionScript`)