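; Base weapon actor that can be equipped, fired and reloaded, setting its mesh and material from its weapon type on BeginPlay.
; Shooting spawns a bullet at the gun muzzle, aimed at the user's shooting vector, and spends magazine ammo; full-auto re-calls StartShoot after a fire-rate delay while shooting continues.
; Reloading refills the magazine from reserve ammo, AddAmmo caps the reserve and returns leftovers, and getters expose ammo and type info.
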(event `self.ReceiveBeginPlay`
  (bind _graphics (`self.Graphics`))
  (set `self.GunEnd` (`self.GunEndArrow`))
  (switch `/Game/WeaponSystem/Enums/E_WeaponType` (`self.WeaponType`)
    (:`NewEnumerator0`
      (`StaticMeshComponent.SetStaticMesh` _graphics "/Game/Models/LP_LiteWeapons_JC/Models/SM_SciFi_Weapons_02.SM_SciFi_Weapons_02")
      (`PrimitiveComponent.SetMaterial` _graphics 0 "/Engine/VREditor/BasicMeshes/MI_Cube_03.MI_Cube_03"))
    (:`NewEnumerator1`
      (`StaticMeshComponent.SetStaticMesh` _graphics "/Game/Weapons_Free/Meshes/SM_pistol_001.SM_pistol_001")
      (`PrimitiveComponent.SetMaterial` _graphics 0 "/Game/Weapons_Free/Materials/M_Material.M_Material"))))

(event `/Game/WeaponSystem/Interface/Weapons/IWeapon.SetWeaponUserParent`
  (params (Parent :type "/Game/WeaponSystem/Interface/Weapons/IWeaponUser Interface"))
  (set `self.WeaponUser` Parent))

(event `/Game/WeaponSystem/Interface/Weapons/IWeapon.Equipped`
  (bind _output_get (set `self.IsEquipped` true))
  (`SceneComponent.SetHiddenInGame` (`self.Graphics`) (not _output_get) false)
  (`KismetSystemLibrary.PrintString` (`KismetStringLibrary.Concat_StrStr` (`self.WeaponName`) " Equipped")))

(event `/Game/WeaponSystem/Interface/Weapons/IWeapon.Unequipped`
  (bind _output_get (set `self.IsEquipped` false))
  (`SceneComponent.SetHiddenInGame` (`self.Graphics`) (not _output_get) false))

(event `/Game/WeaponSystem/Interface/Weapons/IWeapon.StartShoot`
  (if (`self.IsEquipped`)
    (set `self.IsShooting` true)
    ;[1 1 1] Bullet Amount Check
    (if (> (`self.CurrentAmmoInMag`) 0)
      ;[1 1 1] Create a Bullet
      (bind _returnvalue (`|SpawnActorFromClass` "/Game/WeaponSystem/Bullet/BP_BaseBullet.BP_BaseBullet_C" (`SceneComponent.K2_GetComponentToWorld` (`self.GunEnd`)) "AlwaysSpawn" "OverrideRootScale" null (`self.AmmoType`) null))
      ;[1 1 1] Give the Bullet Info
      (bind _dircetion (`/Game/WeaponSystem/Interface/Weapons/IWeaponUser.GetShootingVector` (`self.WeaponUser`) (`self.Range`)))
      (`/Game/WeaponSystem/Bullet/BP_BaseBullet.SetBulletInfoAndShoot` _returnvalue (`self.BulletInfo`) (`KismetMathLibrary.GetDirectionUnitVector` (`SceneComponent.K2_GetComponentLocation` (`self.GunEnd`)) _dircetion))
      ;[1 1 1] Reduce Bullet Amount
      (bind _output_get (set `self.CurrentAmmoInMag` (- (`self.CurrentAmmoInMag`) 1)))
      (`KismetSystemLibrary.PrintString` (`KismetStringLibrary.Conv_IntToString` _output_get) true true (struct :`G` 0.66 :`B` 1.0 :`A` 1.0) 2.0 "Mag")
      ;[1 1 1] calculation of how much time to wait between bullets
      (if (`self.IsFullAuto`)
        ;[1 1 1] if still trying to shoot by the end of the delay call function again
        (`KismetSystemLibrary.Delay` (/ 1.0 (/ (`self.BulletsPerMinutes`) 60.0)))
        (if (`self.IsShooting`)
          (`/Game/WeaponSystem/Interface/Weapons/IWeapon.StartShoot`)))
      (else
        (`KismetSystemLibrary.PrintString` "Need Reload!!!" true true (struct :`R` 1.0 :`B` 0.010841 :`A` 1.0) 2.0 "Mag")
        (set `self.IsShooting` false)))))

(event `/Game/WeaponSystem/Interface/Weapons/IWeapon.StopShoot`
  (set `self.IsShooting` false))

(event `/Game/WeaponSystem/Interface/Weapons/IWeapon.Reload`
  (`self.ReloadLogic`))

(fn `AddAmmo`
  (params (AmountToAdd :type Integer))
  (returns (CanTakeAll :type Boolean) (Leftover :type Integer))
  (bind _returnvalue (+ AmountToAdd (`self.OverAllCurrentAmmo`)))
  (bind _output_get (set `self.Leftovers` (- _returnvalue (`self.MaxOverAllAmmo`))))
  (if (< _returnvalue (`self.MaxOverAllAmmo`))
    (set `self.OverAllCurrentAmmo` _returnvalue)
    (return true 0)
    (else
      (set `self.OverAllCurrentAmmo` (`self.MaxOverAllAmmo`))
      (return false _output_get))))

(fn `CanReload`
  (returns (CanReload :type Boolean))
  (return (> (`self.OverAllCurrentAmmo`) 0)))

(fn `CanShoot`
  (returns (CanShoot :type Boolean))
  (return (> (`self.CurrentAmmoInMag`) 0)))

(fn `GetAmmoInfo`
  (returns (CurrentAmmo :type Integer) (TotalAmmo :type Integer) (MaxInMag :type Integer) (MaxOverall :type Integer) (ReloadTime :type "Float (double-precision)"))
  (return (`self.CurrentAmmoInMag`) (`self.OverAllCurrentAmmo`) (`self.MaxAmmoPerMag`) (`self.MaxOverAllAmmo`) (`self.RelaodTime`)))

(fn `GetAmmoType`
  (returns (AmmoType :type "/Game/WeaponSystem/Enums/E_AmmoType Enum"))
  (return (`self.AmmoType`)))

(fn `GetWeaponType`
  (returns (WeaponType :type "/Game/WeaponSystem/Enums/E_WeaponType Enum"))
  (return (`self.WeaponType`)))

(fn `ReloadLogic`
  ;[1 1 1] Addition of Current and Overall Ammo
  (bind _output_get (set `self.OverAllCurrentAmmo` (+ (`self.CurrentAmmoInMag`) (`self.OverAllCurrentAmmo`))))
  ;[1 1 1] Check Sufficient for Full Amount
  (if (>= _output_get (`self.MaxAmmoPerMag`))
    ;[1 1 1] Reload and Reduce from Current
    (set `self.CurrentAmmoInMag` (`self.MaxAmmoPerMag`))
    (set `self.OverAllCurrentAmmo` (- (`self.OverAllCurrentAmmo`) (`self.MaxAmmoPerMag`)))
    (`KismetSystemLibrary.PrintString` "Reloading..." true true (struct :`R` 0.214985 :`G` 1.0 :`B` 0.04924 :`A` 1.0) 2.0 "Mag" :!label _label)
    (else
      ;[1 1 1] Check if More Than 0
      (if (> (`self.OverAllCurrentAmmo`) 0)
        ;[1 1 1] Unload it All to Magazine and Set to 0
        (set `self.CurrentAmmoInMag` (`self.OverAllCurrentAmmo`))
        (set `self.OverAllCurrentAmmo` 0)
        (goto _label)
        (else
          (`KismetSystemLibrary.PrintString` "No More Bullets!!!" true true (struct :`R` 1.0 :`G` 0.010461 :`B` 0.006999 :`A` 1.0) 5.0 "Mag"))))))

(fn `UserConstructionScript`)