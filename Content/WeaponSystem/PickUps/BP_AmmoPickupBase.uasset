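; Base ammo pickup actor for the weapon system, holding an ammo type and amount.
; On BeginPlay it unhides itself, assigns a sci-fi weapon mesh and switches on the ammo type, with a single emissive material assignment shown.
; GetPickUpData exposes the ammo type, and SetLeftovers overwrites the stored amount with what remains.
; Pickup detection and granting of ammo are not handled in these graphs.
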(event `self.ReceiveBeginPlay`
  (`self.SetActorHiddenInGame` false)
  (`StaticMeshComponent.SetStaticMesh` (`self.StaticMesh`) "/Game/Models/LP_LiteWeapons_JC/Models/SM_SciFi_Weapons_03.SM_SciFi_Weapons_03")
  (switch `/Game/WeaponSystem/Enums/E_AmmoType` (`self.AmmoType`)
    (:`NewEnumerator1`
      (`PrimitiveComponent.SetMaterial` (`self.StaticMesh`) 0 "/Game/Models/Kataan/M_EmissiveO.M_EmissiveO"))))

(fn `GetPickUpData`
  (returns (PickupType :type "/Game/WeaponSystem/Enums/E_AmmoType Enum"))
  (return (`self.AmmoType`)))

(fn `SetLeftovers`
  (params (Leftovers :type Integer))
  (set `self.AmmoAmount` Leftovers))

(fn `UserConstructionScript`)