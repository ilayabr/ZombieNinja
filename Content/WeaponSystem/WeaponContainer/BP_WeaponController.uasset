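; Weapon controller that manages a user's weapons, relaying shoot, reload and swap calls to the equipped one through the IWeapon interface.
; On BeginPlay it claims every BP_WeaponBaseClass actor in the world as its own, maps them by weapon type and equips a default.
; Matching ammo pickups feed only the equipped weapon, with any leftover returned to the pickup.
; Shooting vectors come from the Controller passed to Instantiate.
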(event `self.ReceiveBeginPlay`
  (bind _outactors (`GameplayStatics.GetAllActorsOfClass` "/Game/WeaponSystem/Weapons/BP_WeaponBaseClass.BP_WeaponBaseClass_C"))
  ;[1 1 1] Input All Weapon Actors Into a Map With WeaponType as Key
  (for _array_element _outactors
    (bind _asiweapon (cast `/Game/WeaponSystem/Interface/Weapons/IWeapon` _array_element))
    (`/Game/WeaponSystem/Interface/Weapons/IWeapon.Unequipped` _asiweapon)
    (bind _asiweapon_user (cast `/Game/WeaponSystem/Interface/Weapons/IWeaponUser` self))
    (`/Game/WeaponSystem/Interface/Weapons/IWeapon.SetWeaponUserParent` _asiweapon _asiweapon_user)
    (bind _weapontype (`/Game/WeaponSystem/Interface/Weapons/IWeapon.GetWeaponType` _asiweapon))
    (`BlueprintMapLibrary.Map_Add` (`self.IWeaponTypeMap`) _weapontype _asiweapon))
  (`/Game/WeaponSystem/Interface/Input/IInput.SwapWeapon` "NewEnumerator1"))

(event `/Game/WeaponSystem/Interface/Input/IInput.SwapWeapon`
  (params (WeaponToSwapTo :type "/Game/WeaponSystem/Enums/E_WeaponType Enum" :default "NewEnumerator0"))
  (bind (_value _returnvalue) (`BlueprintMapLibrary.Map_Find` (`self.IWeaponTypeMap`) "NewEnumerator1"))
  (bind (_value_2 _returnvalue_2) (`BlueprintMapLibrary.Map_Find` (`self.IWeaponTypeMap`) WeaponToSwapTo))
  (if (`self.HasWeapon`)
    (bind _weapontype (`/Game/WeaponSystem/Interface/Weapons/IWeapon.GetWeaponType` (`self.EquippedWeapon`)))
    (if (`|EnumEquality` _weapontype WeaponToSwapTo)
      _
      (elif _returnvalue_2
        (`/Game/WeaponSystem/Interface/Weapons/IWeapon.Unequipped` (`self.EquippedWeapon`))
        (`/Game/WeaponSystem/Interface/Weapons/IWeapon.Equipped` _value_2)
        (set `self.EquippedWeapon` _value_2)))
    (elif _returnvalue
      (`/Game/WeaponSystem/Interface/Weapons/IWeapon.Equipped` _value)
      (set `self.HasWeapon` true)
      (set `self.EquippedWeapon` _value))))

(event `/Game/WeaponSystem/Interface/Input/IInput.StartUse`
  ;[1 1 1] Shooting
  (if (`self.HasWeapon`)
    (`/Game/WeaponSystem/Interface/Weapons/IWeapon.StartShoot` (`self.EquippedWeapon`))))

(event `/Game/WeaponSystem/Interface/Input/IInput.StopUse`
  ;[1 1 1] Shooting
  (if (`self.HasWeapon`)
    (`/Game/WeaponSystem/Interface/Weapons/IWeapon.StopShoot` (`self.EquippedWeapon`))))

(event `/Game/WeaponSystem/Interface/Input/IInput.Reload`
  ;[1 1 1] Reload
  (if (`self.HasWeapon`)
    (`/Game/WeaponSystem/Interface/Weapons/IWeapon.Reload` (`self.EquippedWeapon`))))

(event `/Game/WeaponSystem/Interface/Pickup/IPickuper.NotifyOverlapWithPickUp`
  (params (PickableObj :type "/Game/WeaponSystem/PickUps/BP_PickUpBase Object Reference"))
  (bind _equippedweapon (`self.EquippedWeapon`))
  (bind _asbp_ammo_pickup_base (cast `/Game/WeaponSystem/PickUps/BP_AmmoPickupBase` PickableObj))
  (if (`self.HasWeapon`)
    ;[1 1 1] equipped weapon add ammo
    (bind _ammotype (`/Game/WeaponSystem/Interface/Weapons/IWeapon.GetAmmoType` _equippedweapon))
    (if (`|EnumEquality` _ammotype (`/Game/WeaponSystem/PickUps/BP_AmmoPickupBase.AmmoType` _asbp_ammo_pickup_base))
      (bind (_cantakeall _leftover) (`/Game/WeaponSystem/Interface/Weapons/IWeapon.AddAmmo` _equippedweapon (`/Game/WeaponSystem/PickUps/BP_AmmoPickupBase.AmmoAmount` _asbp_ammo_pickup_base)))
      ;[1 1 1] send back leftover ammo that didnt fit in the mag
      (if _cantakeall
        (`/Game/WeaponSystem/PickUps/BP_PickUpBase.WasPickedUp` _asbp_ammo_pickup_base)
        (else
          (`/Game/WeaponSystem/PickUps/BP_AmmoPickupBase.SetLeftovers` _asbp_ammo_pickup_base _leftover))))))

(event `/Game/WeaponSystem/Interface/Input/IInput.Instantiate`
  (params (Controller :type "/Game/Blueprint/Player/BP_PlayerStateMachine Object Reference"))
  (set `self.Controller` Controller))

(fn `CheckCanUse`
  (returns (CanUse :type Boolean))
  (if (`self.HasWeapon`)
    (bind _canshoot (`/Game/WeaponSystem/Interface/Weapons/IWeapon.CanShoot` (`self.EquippedWeapon`)))
    (return _canshoot)
    (else
      (return false))))

(fn `CheckReload`
  (returns (CanReload :type Boolean))
  (if (`self.HasWeapon`)
    (bind _canreload (`/Game/WeaponSystem/Interface/Weapons/IWeapon.CanReload` (`self.EquippedWeapon`)))
    (return _canreload)
    (else
      (return false))))

(fn `GetShootingVector`
  (params (EffectiveRange :type "Float (double-precision)"))
  (returns (Dircetion :type "Vector Structure"))
  (bind _dircetion (`/Game/Blueprint/Player/BP_PlayerStateMachine.GetShootingVector` (`self.Controller`) EffectiveRange))
  (return _dircetion))

(fn `SetEquippedWeapon`)

(fn `UnequipLast`
  (if (`self.HasWeapon`)
    (`/Game/WeaponSystem/Interface/Weapons/IWeapon.Unequipped` (`self.EquippedWeapon`))))

(fn `UserConstructionScript`)