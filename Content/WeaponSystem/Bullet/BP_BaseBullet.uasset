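; BP_BaseBullet is the base bullet actor of the weapon system, a physics-driven projectile with a short lifetime.
; SetBulletInfoAndShoot stores the bullet info, applies its size and gravity setting, unhides the actor and launches BulletGraphics with a force-scaled impulse along the given direction.
; BeginPlay has an AmmoType switch with no case logic shown, and a one-second delay before the actor destroys itself.
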(event `self.ReceiveBeginPlay`
  (switch `/Game/WeaponSystem/Enums/E_AmmoType` (`self.AmmoType`)
    (:`NewEnumerator1`
      (`KismetSystemLibrary.Delay` 1.0)
      (`self.K2_DestroyActor`))))

(fn `SetBulletInfoAndShoot`
  (params (BulletInfo :type "/Game/WeaponSystem/Structs/S_BulletInfo Structure") (Direction :type "Vector Structure"))
  (bind _output_get (set `self.BulletInfo` BulletInfo))
  (`self.SetActorRelativeScale3D` (`KismetMathLibrary.MakeVector` (`.Size_19_525D6F87410B1A5A61702795A743F459` (break `/Game/WeaponSystem/Structs/S_BulletInfo` _output_get)) (`.Size_19_525D6F87410B1A5A61702795A743F459` (break `/Game/WeaponSystem/Structs/S_BulletInfo` _output_get)) (`.Size_19_525D6F87410B1A5A61702795A743F459` (break `/Game/WeaponSystem/Structs/S_BulletInfo` _output_get))))
  (`PrimitiveComponent.SetEnableGravity` (`self.BulletGraphics`) (`.IsGravity_21_C4EDC597426AAB6B106DC3B9672A3D85` (break `/Game/WeaponSystem/Structs/S_BulletInfo` _output_get)))
  (`self.SetActorHiddenInGame` false)
  (`PrimitiveComponent.AddImpulse` (`self.BulletGraphics`) (* Direction (break `/Game/WeaponSystem/Structs/S_BulletInfo` _output_get)) "None" false))

(fn `UserConstructionScript`)