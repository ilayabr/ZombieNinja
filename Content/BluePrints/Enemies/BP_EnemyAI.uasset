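; Enemy AI controller that runs a Patrol, Look At and Chase state machine on Tick against the first player's pawn.
; Patrol loops through externally supplied points, resuming at the closest, with moves triggered through an event dispatcher.
; A player in range stops the enemy, which turns toward them for a timed look, then chases if still in range.
; Chase follows until its timer expires, regardless of distance, then returns to patrol.
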(event `self.ReceiveBeginPlay`
  (set `self.TargetPlayer` (`GameplayStatics.GetPlayerPawn` 0))
  (set `self.PossesedPawn` (`self.K2_GetPawn`))
  (add `self.SetAiMoveTo` (delegate `SetAiMoveTo_Event`))
  (`self.PatrolOnEnter`))

(event `SetAiMoveTo_Event`
  (if (`self.HasPatrolPoints`)
    (`|AIMoveTo` (`self.PossesedPawn`) (0.0 0.0 0.0) (`|GetArrayItem` (`self.PatrolPoints`) (`self.PatrolPointIndex`)))))

(event `self.ReceiveTick`
  (params (DeltaSeconds :type "Float (single-precision)"))
  (`self.CheckForNextState`)
  (switch `/Game/Enums/E_EnemyState` (`self.AiState`)
    (:`NewEnumerator0`
      (`self.PatrolTick` DeltaSeconds))
    (:`NewEnumerator1`
      (`self.LookAtTick` DeltaSeconds))
    (:`NewEnumerator2`
      (`self.ChaseTick` DeltaSeconds)
      (`|AIMoveTo` (`self.PossesedPawn`) (0.0 0.0 0.0) (`self.TargetPlayer`) 4.0 true))))

(fn `ChaseTick`
  (params (`delta time` :type "Float (double-precision)"))
  (set `self.ChaseTimer` (+ `delta time` (`self.ChaseTimer`))))

(fn `CheckForNextState`
  (switch `/Game/Enums/E_EnemyState` (`self.AiState`)
    (:`NewEnumerator0`
      (if (`self.CheckTragetDistanceInRange`)
        (`self.StopMovement`)
        (set `self.AiState` "NewEnumerator1")))
    (:`NewEnumerator1`
      (if (>= (`self.LookAtTimer`) (`self.LookAtMaxTimer`))
        (set `self.LookAtTimer` 0.0)
        (if (`self.CheckTragetDistanceInRange`)
          (set `self.AiState` "NewEnumerator2")
          (else
            (set `self.AiState` "NewEnumerator0")
            (`self.PatrolOnEnter`)))))
    (:`NewEnumerator2`
      ; check follow timer
      (if (>= (`self.ChaseTimer`) (`self.ChaseMaxTimer`))
        (set `self.AiState` "NewEnumerator0")
        (set `self.ChaseTimer` 0.0)
        (`self.StopMovement`)
        (`self.PatrolOnEnter`)))))

(fn `CheckTragetDistanceInRange`
  (returns (IsInRange :type Boolean))
  (return (< (`KismetMathLibrary.Vector_Distance` (`self.K2_GetActorLocation` (`self.PossesedPawn`)) (`self.K2_GetActorLocation` (`self.TargetPlayer`))) (`self.MinDistance`))))

(fn `GetClosestPatrolPointIndexInArray`
  (params (Array :type "Array of Actor Object Reference")))

(fn `LookAtTick`
  (params (`delta time` :type "Float (double-precision)"))
  (bind (_returnvalue_roll _returnvalue_pitch _returnvalue_yaw) (`KismetMathLibrary.BreakRotator` (`KismetMathLibrary.RLerp` (`self.K2_GetActorRotation` (`self.PossesedPawn`)) (`KismetMathLibrary.FindLookAtRotation` (`self.K2_GetActorLocation` (`self.PossesedPawn`)) (`self.K2_GetActorLocation` (`self.TargetPlayer`))) (* `delta time` (`self.RotationSpeed`)) true)))
  ; Increment Timer
  (set `self.LookAtTimer` (+ `delta time` (`self.LookAtTimer`)))
  ; Rotate Enemy to Look At Player
  (`self.K2_SetActorRotation` (`self.PossesedPawn`) (`KismetMathLibrary.MakeRotator` _returnvalue_roll 0.0 _returnvalue_yaw) false))

(fn `OnPatrolPointReached`
  (bind _result (`/Engine/EditorBlueprintResources/StandardMacros.IncrementInt` (`self.PatrolPointIndex`))
    (:`  `
      (set `self.PatrolPointIndex` (mod _result (`KismetArrayLibrary.Array_Length` (`self.PatrolPoints`))))
      (`self.SetAiMoveTo`))))

(fn `PatrolOnEnter`
  (if (`self.HasPatrolPoints`)
    (for (_ _array_index) (`self.PatrolPoints`)
      (if (<= (`KismetMathLibrary.Vector_Distance` (`self.K2_GetActorLocation` (`self.K2_GetPawn`)) (`self.K2_GetActorLocation` (`|GetArrayItem` (`self.PatrolPoints`) _array_index))) (`KismetMathLibrary.Vector_Distance` (`self.K2_GetActorLocation` (`self.K2_GetPawn`)) (`self.K2_GetActorLocation` (`|GetArrayItem` (`self.PatrolPoints`) (`self.ShortestDistanceIndex`)))))
        (set `self.ShortestDistanceIndex` _array_index)))
    (set `self.PatrolPointIndex` (`self.ShortestDistanceIndex`))
    (`self.SetAiMoveTo`)))

(fn `PatrolTick`
  (params (`delta time` :type "Float (double-precision)"))
  (if (`self.HasPatrolPoints`)
    (if (<= (`KismetMathLibrary.Vector_Distance` (`self.K2_GetActorLocation` (`|GetArrayItem` (`self.PatrolPoints`) (`self.PatrolPointIndex`))) (`self.K2_GetActorLocation` (`self.PossesedPawn`))) (`self.PatrolPointMinimumDistance`))
      (`self.StopMovement`)
      (`self.OnPatrolPointReached`))))

(fn `SetPatrolPoints`
  (params (PatrolPoints :type "Array of Actor Object Reference"))
  (set `self.PatrolPoints` PatrolPoints)
  (set `self.HasPatrolPoints` true)
  (`self.SetAiMoveTo`))

(fn `UserConstructionScript`)