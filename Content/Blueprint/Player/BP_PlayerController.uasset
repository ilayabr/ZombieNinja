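; Player controller that adds the Cowmurai Enhanced Input mapping context and turns player input into generic notifications.
; Grenade, aim, attack, reload, jump, dash, sprint and move actions report performed or canceled with an enum value identifying the action.
; While CanMove is set, move input broadcasts its vector and drives the pawn cached at BeginPlay along world axes.
; Look input is broadcast as a rotator with Y inverted, without rotating anything here.
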(event `self.ReceiveBeginPlay`
  (`EnhancedInputSubsystemInterface.AddMappingContext` (subsystem `EnhancedInputLocalPlayerSubsystem`) "/Game/Blueprint/Input/IMC_CowmuraiMap.IMC_CowmuraiMap" 0 (struct))
  (set `self.PlayerPawn` (`GameplayStatics.GetPlayerPawn` 0)))

(event `EnhancedInput|/Game/Blueprint/Input/IA_GrenadeThrow`
  (params (ActionValue :type Boolean) (ElapsedSeconds :type "Float (double-precision)") (TriggeredSeconds :type "Float (double-precision)") (InputAction :type "InputAction Object Reference" :default "/Game/Blueprint/Input/IA_GrenadeThrow.IA_GrenadeThrow"))
  ; GrenadeInput
  (:`Started`
    (`self.OnInputPerformed` "NewEnumerator11"))
  (:`Canceled`
    (`self.OnInputCanceled` "NewEnumerator11" :!label _label))
  (:`Completed`
    (goto _label)))

(event `EnhancedInput|/Game/Blueprint/Input/IA_Aim`
  (params (ActionValue :type Boolean) (ElapsedSeconds :type "Float (double-precision)") (TriggeredSeconds :type "Float (double-precision)") (InputAction :type "InputAction Object Reference" :default "/Game/Blueprint/Input/IA_Aim.IA_Aim"))
  ; AimInput
  (:`Started`
    (`self.OnInputPerformed` "NewEnumerator5"))
  (:`Canceled`
    (`self.OnInputCanceled` "NewEnumerator5" :!label _label_2))
  (:`Completed`
    (goto _label_2)))

(event `EnhancedInput|/Game/Blueprint/Input/IA_Attack`
  (params (ActionValue :type Boolean) (ElapsedSeconds :type "Float (double-precision)") (TriggeredSeconds :type "Float (double-precision)") (InputAction :type "InputAction Object Reference" :default "/Game/Blueprint/Input/IA_Attack.IA_Attack"))
  ; Attack Input
  (:`Started`
    (`self.OnInputPerformed` "NewEnumerator4"))
  (:`Canceled`
    (`self.OnInputCanceled` "NewEnumerator4" :!label _label_3))
  (:`Completed`
    (goto _label_3)))

(event `EnhancedInput|/Game/Blueprint/Input/IA_Reload`
  (params (ActionValue :type Boolean) (ElapsedSeconds :type "Float (double-precision)") (TriggeredSeconds :type "Float (double-precision)") (InputAction :type "InputAction Object Reference" :default "/Game/Blueprint/Input/IA_Reload.IA_Reload"))
  ; DashInput
  (:`Started`
    (`self.OnInputPerformed` "NewEnumerator8"))
  (:`Canceled`
    (`self.OnInputCanceled` "NewEnumerator8" :!label _label_4))
  (:`Completed`
    (goto _label_4)))

(event `EnhancedInput|/Game/Blueprint/Input/IA_Move`
  (params (ActionValue :type "Vector2D Structure") (ElapsedSeconds :type "Float (double-precision)") (TriggeredSeconds :type "Float (double-precision)") (InputAction :type "InputAction Object Reference" :default "/Game/Blueprint/Input/IA_Move.IA_Move"))
  ; MoveInput
  (:`Triggered`
    (set `self.MoveVector` (`KismetMathLibrary.MakeVector` ActionValue_X ActionValue_Y) :!label _label_5)
    (if (`self.CanMove`)
      (`self.OnMoveVectorChanged` (`self.MoveVector`))
      (`Pawn.AddMovementInput` (`self.PlayerPawn`) (`self.MoveVector`) 1.0 false)))
  (:`Started`
    (`self.OnInputPerformed` "NewEnumerator0")
    (goto _label_5))
  (:`Completed`
    (`self.OnInputCanceled` "NewEnumerator0")
    (set `self.MoveVector` (0.0 0.0 0.0))))

(event `EnhancedInput|/Game/Blueprint/Input/IA_Jump`
  (params (ActionValue :type Boolean) (ElapsedSeconds :type "Float (double-precision)") (TriggeredSeconds :type "Float (double-precision)") (InputAction :type "InputAction Object Reference" :default "/Game/Blueprint/Input/IA_Jump.IA_Jump"))
  ; JumpInput
  (:`Started`
    (`self.OnInputPerformed` "NewEnumerator3"))
  (:`Canceled`
    (`self.OnInputCanceled` "NewEnumerator3" :!label _label_6))
  (:`Completed`
    (goto _label_6)))

(event `EnhancedInput|/Game/Blueprint/Input/IA_Dash`
  (params (ActionValue :type Boolean) (ElapsedSeconds :type "Float (double-precision)") (TriggeredSeconds :type "Float (double-precision)") (InputAction :type "InputAction Object Reference" :default "/Game/Blueprint/Input/IA_Dash.IA_Dash"))
  ; Dash Input
  (:`Started`
    (`self.OnInputPerformed` "NewEnumerator7"))
  (:`Canceled`
    (`self.OnInputCanceled` "NewEnumerator7" :!label _label_7))
  (:`Completed`
    (goto _label_7)))

(event `EnhancedInput|/Game/Blueprint/Input/IA_Sprint`
  (params (ActionValue :type Boolean) (ElapsedSeconds :type "Float (double-precision)") (TriggeredSeconds :type "Float (double-precision)") (InputAction :type "InputAction Object Reference" :default "/Game/Blueprint/Input/IA_Sprint.IA_Sprint"))
  ; Sprint Input
  (:`Started`
    (`self.OnInputPerformed` "NewEnumerator6"))
  (:`Canceled`
    (`self.OnInputCanceled` "NewEnumerator6" :!label _label_8))
  (:`Completed`
    (goto _label_8)))

(event `EnhancedInput|/Game/Blueprint/Input/IA_Look`
  (params (ActionValue :type "Vector2D Structure") (ElapsedSeconds :type "Float (double-precision)") (TriggeredSeconds :type "Float (double-precision)") (InputAction :type "InputAction Object Reference" :default "/Game/Blueprint/Input/IA_Look.IA_Look"))
  (:`Triggered`
    (bind _output_get (set `self.Rotator` (`KismetMathLibrary.MakeRotator` 0.0 (* ActionValue_Y -1.0) ActionValue_X)))
    (`self.OnLookVectorChanged` _output_get)))

(fn `UserConstructionScript`)