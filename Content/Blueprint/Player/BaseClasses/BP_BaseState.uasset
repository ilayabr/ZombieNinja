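; Base class for player states, giving derived states shared enter, tick and exit behavior within an owning state machine.
; Entering resets exit permission and timer, then sets movement, speed and aim camera through the state machine from per-state flags.
; Timed states count up while active, then unlock exit and signal that the state ended.
; Entry check defaults to false, exit check returns the can-change flag.
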(event `/Game/Blueprint/Player/Interfaces/IState.Initialize`
  (params (StateMachine :type "/Game/Blueprint/Player/BP_PlayerStateMachine Object Reference"))
  (set `self.StateMachine` StateMachine))

(event `/Game/Blueprint/Player/Interfaces/IState.ControlledTick`
  (params (DeltaTime :type "Float (double-precision)"))
  ; basic implementation of class
  (`self.BaseTick` DeltaTime))

(event `/Game/Blueprint/Player/Interfaces/IState.OnExit`
  ; basic implementation of class
  (`self.BaseOnExit`))

(event `/Game/Blueprint/Player/Interfaces/IState.BaseTick`
  (params (DeltaTime :type "Float (double-precision)"))
  ; if has timer and the state active start counting the seconds
  (if (`self.IsTimedState`)
    (if (`self.StateActive`)
      (bind _output_get (set `self.InStateTimer` (+ DeltaTime (`self.InStateTimer`))))
      (if (>= _output_get (`self.MaxTimeInState`))
        (set `self.CanChangeState` true)
        (`self.StateEnded`)))))

(event `/Game/Blueprint/Player/Interfaces/IState.OnEnter`
  ; basic implementation of class
  (`self.BaseOnEnter`))

(event `/Game/Blueprint/Player/Interfaces/IState.BaseOnExit`
  ; exit
  (set `self.StateActive` false))

(event `/Game/Blueprint/Player/Interfaces/IState.BaseOnEnter`
  (bind _statemachine (`self.StateMachine`))
  (bind _statemachine_2 (`self.StateMachine`))
  (bind _statemachine_3 (`self.StateMachine`))
  ; Enter
  (`|ExecutionSequence`
    (:`then_0`
      ;; movement Control
      (if (`self.IsMovingState`)
        (`/Game/Blueprint/Player/BP_PlayerStateMachine.SetCanMove` _statemachine_3 true)
        (`/Game/Blueprint/Player/BP_PlayerStateMachine.SetSpeed` _statemachine_3 (`self.MoveSpeed`))
        (else
          (`/Game/Blueprint/Player/BP_PlayerStateMachine.SetCanMove` _statemachine_2 false)
          (`/Game/Blueprint/Player/BP_PlayerStateMachine.SetSpeed` _statemachine_2 0.0))))
    (:`then_1`
      ;; Reset variables
      (if true
        (set `self.CanChangeState` false)
        (set `self.InStateTimer` 0.0)
        (set `self.StateActive` true)
        (else
          (set `self.CanChangeState` true))))
    (:`then_2`
      ;; CameraControl
      (if (`self.IsAimedState`)
        (`/Game/Blueprint/Player/BP_PlayerStateMachine.OnPlayerAimedEvent` _statemachine)
        (else
          (`/Game/Blueprint/Player/BP_PlayerStateMachine.OnPlayerNotAimingEvent` _statemachine))))))

(fn `CheckEntryCondition`
  (returns (CanEnter :type Boolean))
  (return false))

(fn `CheckExitCondition`
  (returns (CanExit :type Boolean))
  (return (`self.CanChangeState`)))

(fn `UserConstructionScript`)