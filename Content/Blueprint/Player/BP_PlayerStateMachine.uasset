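; Player character Blueprint that runs a state machine over BP_BaseState actors gathered from the level at BeginPlay.
; Controller input events update a context map; then the current state's exit check gates entry-checked transitions, falling back to any-state transitions.
; It ticks the active state and provides movement impulses, box-trace sword attacks and camera line-trace shots with headshot detection against zombies.
; Timelines lerp the camera between default and aimed positions.
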(event `OnPlayerAimedEvent`
  (`|ExecutionSequence`
    (:`then_0`
      ;[1 1 1] Transition to non aimed camera
      (bind (_direction _newtrack_0) (`Timeline|CameraToOrigin` :!via `Stop` :!label _label)
        (:`Update`
          (`SceneComponent.K2_SetWorldLocation` (`self.MainCamera`) (`KismetMathLibrary.VLerp` (`SceneComponent.K2_GetComponentLocation` (`self.MainCamera`)) (`SceneComponent.K2_GetComponentLocation` (`self.Origin Position`)) _newtrack_0) false false))))
    (:`then_1`
      ;[1 1 1] Transition to aimed camera
      (bind (_direction_2 _newtrack_0_2) (`Timeline|CameraToAimed` :!via `PlayFromStart` :!label _label_2)
        (:`Update`
          (`SceneComponent.K2_SetWorldLocation` (`self.MainCamera`) (`KismetMathLibrary.VLerp` (`SceneComponent.K2_GetComponentLocation` (`self.MainCamera`)) (`SceneComponent.K2_GetComponentLocation` (`self.Aimed Position`)) _newtrack_0_2) false false))))))

(event `OnPlayerNotAimingEvent`
  (`|ExecutionSequence`
    (:`then_0`
      (goto _label_2 :!via `Stop`))
    (:`then_1`
      (goto _label :!via `PlayFromStart`))))

(event `OnLookChangedEvent`
  (params (LookInput :type "Rotator Structure"))
  (bind (_relativerotation_roll _relativerotation_pitch) (`KismetMathLibrary.BreakRotator` (`SceneComponent.RelativeRotation` (`self.Axis Position`))))
  ; LookAround
  (`self.K2_AddActorLocalRotation` (`KismetMathLibrary.MakeRotator` 0.0 0.0 LookInput_Yaw))
  ;; clamp rotation.....
  (if (> LookInput_Pitch 0.0)
    (if (not (>= _relativerotation_pitch 20.0))
      (`SceneComponent.K2_AddRelativeRotation` (`self.Axis Position`) (`KismetMathLibrary.MakeRotator` 0.0 LookInput_Pitch) false false :!label _label_3))
    (elif (not (<= _relativerotation_pitch -20.0))
      (goto _label_3))))

(event `self.ReceiveBeginPlay`
  (bind _returnvalue (`|CreateWidget` "/Game/UI/MainGameUI.MainGameUI_C"))
  (`UserWidget.AddToViewport` _returnvalue 0)
  ;[1 1 1] Get Controller And listen to events
  (bind _returnvalue_2 (`GameplayStatics.GetActorOfClass` "/Game/Blueprint/Player/BP_PlayerController.BP_PlayerController_C"))
  (bind _output_get (set `self.PlayerController` _returnvalue_2))
  (bind _returnvalue_3 (`GameplayStatics.GetActorOfClass` "/Game/WeaponSystem/WeaponContainer/BP_WeaponController.BP_WeaponController_C"))
  (bind _output_get_2 (set `self.WeaponController` _returnvalue_3))
  (`/Game/WeaponSystem/Interface/Input/IInput.Instantiate` _output_get_2 self)
  ; Event Subscription
  (add `/Game/Blueprint/Player/BP_PlayerController.OnInputCanceled` _output_get (delegate `OnInputCanceledEvent`))
  (add `/Game/Blueprint/Player/BP_PlayerController.OnInputPerformed` _output_get (delegate `OnInputPerformedEvent`))
  (add `self.OnPlayerAiming` (delegate `OnPlayerAimedEvent`))
  (add `self.OnPlayerNotAiming` (delegate `OnPlayerNotAimingEvent`))
  (add `/Game/Blueprint/Player/BP_PlayerController.OnLookVectorChanged` (`self.PlayerController`) (delegate `OnLookChangedEvent`))
  (`self.LerpCameraToOrigin`)
  ;[1 1 1] Get All States from heitrarchy and instantiate idle default
  (bind _outactors (`GameplayStatics.GetAllActorsOfClass` "/Game/Blueprint/Player/BaseClasses/BP_BaseState.BP_BaseState_C"))
  (for _array_element _outactors
    (`BlueprintMapLibrary.Map_Add` (`self.StateMap`) (`/Game/Blueprint/Player/BaseClasses/BP_BaseState.StateType` _array_element) _array_element)
    (`/Game/Blueprint/Player/Interfaces/IState.Initialize` _array_element self)
    (add `/Game/Blueprint/Player/BaseClasses/BP_BaseState.StateEnded` _array_element (delegate `StateEndedEvent`)))
  (if (`BlueprintMapLibrary.Map_Contains` (`self.StateMap`) "NewEnumerator1")
    (`self.SetState` "NewEnumerator1")
    ;[1 1 1] Instantiate all input
    (bind _enumvalue (foreach `/Game/Blueprint/Input/Enum/E_InputType` false)
      (:`LoopBody`
        (`BlueprintMapLibrary.Map_Add` (`self.PlayerContextMap`) _enumvalue)))))

(event `OnInputPerformedEvent`
  (params (InputType :type "/Game/Blueprint/Input/Enum/E_InputType Enum" :default "NewEnumerator0"))
  (bind _playercontextmap (`self.PlayerContextMap`))
  ;[1 1 1] INPUT HANDLING
  (if (`BlueprintMapLibrary.Map_Contains` _playercontextmap InputType)
    (`BlueprintMapLibrary.Map_Remove` _playercontextmap InputType))
  (`BlueprintMapLibrary.Map_Add` _playercontextmap InputType true)
  ;;[1 1 1] ExitCheck
  (bind _canexit (`/Game/Blueprint/Player/Interfaces/IState.CheckExitCondition` (`self.CurrentState`) :!label _label_4))
  (if _canexit
    ;[1 1 1] Check Current State Transitions
    (set `self.StateFound` false :!label _label_5)
    (if (`self.IsAlive`)
      (for _array_element (`/Game/Blueprint/Player/BaseClasses/BP_BaseState.StateTransitions` (`self.CurrentState`))
        (bind (_value _returnvalue) (`BlueprintMapLibrary.Map_Find` (`self.StateMap`) _array_element))
        (if _returnvalue
          (bind _canenter (`/Game/Blueprint/Player/Interfaces/IState.CheckEntryCondition` _value))
          (if _canenter
            (bind _statehaschanged (`self.ChangeState` _array_element))
            (if _statehaschanged
              (set `self.StateFound` true)
              (break)))))
      ;[1 1 1] Check Any Transition
      ;; if found state opt out
      (if (not (`self.StateFound`))
        (for _array_element_2 (`self.AnyStateTransition`)
          (bind (_value_2 _returnvalue_2) (`BlueprintMapLibrary.Map_Find` (`self.StateMap`) _array_element_2))
          (if _returnvalue_2
            (bind _canenter_2 (`/Game/Blueprint/Player/Interfaces/IState.CheckEntryCondition` _value_2))
            (if _canenter_2
              (bind _statehaschanged_2 (`self.ChangeState` _array_element_2))
              (if _statehaschanged_2
                (break)))))))))

(event `StateEndedEvent`
  ;[1 1 1] INPUT HANDLING
  (goto _label_5))

(event `OnInputCanceledEvent`
  (params (InputType :type "/Game/Blueprint/Input/Enum/E_InputType Enum" :default "NewEnumerator0"))
  (bind _playercontextmap (`self.PlayerContextMap`))
  ;[1 1 1] INPUT HANDLING
  (if (`BlueprintMapLibrary.Map_Contains` _playercontextmap InputType)
    (`BlueprintMapLibrary.Map_Remove` _playercontextmap InputType))
  (`BlueprintMapLibrary.Map_Add` _playercontextmap InputType)
  (goto _label_4))

(event `self.ReceiveTick`
  (params (DeltaSeconds :type "Float (single-precision)"))
  ;[1 1 1] Tick Logic
  (`/Game/Blueprint/Player/Interfaces/IState.ControlledTick` (`self.CurrentState`) DeltaSeconds))

(event `/Game/WeaponSystem/Interface/Pickup/IPickuper.NotifyOverlapWithPickUp`
  (params (PickableObj :type "/Game/WeaponSystem/PickUps/BP_PickUpBase Object Reference"))
  (`/Game/WeaponSystem/WeaponContainer/BP_WeaponController.NotifyOverlapWithPickUp` (`self.WeaponController`) PickableObj))

(event `/Game/WeaponSystem/Interface/Weapons/IDamageable.DealDamage`
  (params (DamageAmount :type Integer))
  (set `self.HP` (- (`self.HP`) DamageAmount))
  (`self.PlayerGotHit`)
  (if (<= (`self.HP`) 0)
    (`self.PlayerDied`)
    (set `self.IsAlive` false)))

(fn `Attack`
  (params (Damage :type Integer) (`IsSpecial?` :type Boolean))
  (locals (HitActors :type "Set of Actor Object Reference"))
  (bind (_returnvalue_roll _returnvalue_pitch _returnvalue_yaw) (`KismetMathLibrary.BreakRotator` (`self.K2_GetActorRotation`)))
  (bind _returnvalue (`self.K2_GetActorLocation`))
  (bind _range (`self.GetRange` `IsSpecial?`))
  (bind _outhits (`KismetSystemLibrary.BoxTraceMulti` :`Start` _returnvalue :`End` (+ _returnvalue (* _range (`self.GetActorForwardVector`))) :`HalfSize` (10.0 100.0 10.0) :`Orientation` (`KismetMathLibrary.MakeRotator` (`KismetMathLibrary.RandomFloatInRange` 60.0 -60.0) 0.0 _returnvalue_yaw) :`TraceChannel` "TraceTypeQuery1" :`DrawDebugType` "ForDuration"))
  (for _array_element _outhits
    (bind _asbp_base_zombie (cast `/Game/Blueprint/Enemy/BP_BaseZombie` (`.HitActor` (`GameplayStatics.BreakHitResult` _array_element))))
    (if (not (`BlueprintSetLibrary.Set_Contains` (`local.HitActors`) (`.HitActor` (`GameplayStatics.BreakHitResult` _array_element))))
      (`/Game/Blueprint/Enemy/BP_BaseZombie.JumpToChase` _asbp_base_zombie true Damage)
      (`BlueprintSetLibrary.Set_Add` (`local.HitActors`) (`.HitActor` (`GameplayStatics.BreakHitResult` _array_element))))))

(fn `ChangeState`
  (params (NewState :type "/Game/Blueprint/Player/E_StateType Enum" :default "NewEnumerator0"))
  (returns (StateHasChanged :type Boolean))
  (bind (_value _returnvalue) (`BlueprintMapLibrary.Map_Find` (`self.StateMap`) NewState))
  (if _returnvalue
    (if (`|EnumEquality` NewState (`/Game/Blueprint/Player/BaseClasses/BP_BaseState.StateType` (`self.CurrentState`)))
      (`KismetSystemLibrary.PrintString` "I Tried to Get into the same State")
      (return false)
      (else
        (`/Game/Blueprint/Player/Interfaces/IState.OnExit` (`self.CurrentState`))
        (bind _output_get (set `self.CurrentState` _value))
        (`/Game/Blueprint/Player/Interfaces/IState.OnEnter` _output_get)
        (`self.OnStateChanged` NewState)
        (`KismetSystemLibrary.PrintString` (`KismetStringLibrary.Concat_StrStr` (`|GetEnumeratorNameAsString` NewState) "OnEnter") true true (struct :`G` 1.0 :`A` 1.0) 30.0 "State")
        (return true)))
    (else
      (`KismetSystemLibrary.PrintString` "State Not Found" true true (struct :`R` 1.0 :`A` 1.0))
      (return false))))

(fn `GetRange`
  (params (IsSpecial :type Boolean))
  (returns (Range :type "Float (double-precision)"))
  (if IsSpecial
    (return (`self.SpecialRange`))
    (else
      (return (`self.Sword Range`)))))

(fn `GetShootingVector`
  (params (EffectiveRange :type "Float (double-precision)"))
  (returns (Dircetion :type "Vector Structure"))
  (bind _maincamera (`self.MainCamera`))
  (bind _returnvalue (`SceneComponent.K2_GetComponentLocation` _maincamera))
  (bind _returnvalue_2 (+ _returnvalue (* EffectiveRange (`SceneComponent.GetForwardVector` _maincamera))))
  (bind (_outhit _returnvalue_3) (`KismetSystemLibrary.LineTraceSingle` :`Start` _returnvalue :`End` _returnvalue_2 :`TraceChannel` "TraceTypeQuery1" :`DrawDebugType` "ForDuration"))
  (if _returnvalue_3
    (bind (_bblockinghit _binitialoverlap _time _distance _location _impactpoint _normal _impactnormal _physmat _hitactor _hitcomponent) (`GameplayStatics.BreakHitResult` _outhit))
    (bind _asbp_base_zombie (cast `/Game/Blueprint/Enemy/BP_BaseZombie` _hitactor)
      (:`then`
        (if (`KismetStringLibrary.EqualEqual_StrStr` (`KismetSystemLibrary.GetObjectName` _hitcomponent) "HeadCollider")
          (`/Game/Blueprint/Enemy/BP_BaseZombie.JumpToChase` _asbp_base_zombie true 100)
          (else
            (`/Game/Blueprint/Enemy/BP_BaseZombie.JumpToChase` _asbp_base_zombie true 67))))
      (:`CastFailed`
        _))
    (return _impactpoint)
    (else
      (return _returnvalue_2))))

(fn `ImpulseInMoveDirection`
  (params (Force :type "Float (double-precision)"))
  (bind (_returnvalue_x _returnvalue_y) (`KismetMathLibrary.BreakVector` (`self.GetActorForwardVector`)))
  (bind (_returnvalue_x_2 _returnvalue_y_2) (`KismetMathLibrary.BreakVector` (`self.GetActorRightVector`)))
  (bind (_movevector_x _movevector_y) (`KismetMathLibrary.BreakVector` (`/Game/Blueprint/Player/BP_PlayerController.MoveVector` (`self.PlayerController`))))
  (`CharacterMovementComponent.AddImpulse` (`self.CharacterMovement`) (* Force (`KismetMathLibrary.Normal` (+ (* _movevector_x (`KismetMathLibrary.MakeVector` _returnvalue_x _returnvalue_y)) (* _movevector_y (`KismetMathLibrary.MakeVector` _returnvalue_x_2 _returnvalue_y_2))))) true))

(fn `ImpulsePlayerForward`
  (params (Force :type "Float (double-precision)"))
  (bind (_returnvalue_x _returnvalue_y) (`KismetMathLibrary.BreakVector` (`self.GetActorForwardVector`)))
  (`CharacterMovementComponent.AddImpulse` (`self.CharacterMovement`) (* Force (`KismetMathLibrary.MakeVector` _returnvalue_x _returnvalue_y)) true))

(fn `IsGrounded`
  (returns (IsGround :type Boolean))
  (return (`|EnumEquality` (`CharacterMovementComponent.MovementMode` (`self.CharacterMovement`)) "MOVE_Walking")))

(fn `JumpImpulse`
  (params (Force :type "Float (double-precision)"))
  (`CharacterMovementComponent.AddImpulse` (`self.CharacterMovement`) (* Force (`KismetMathLibrary.Vector_Up`)) true))

(fn `LerpCameraToAimed`
  (`self.OnPlayerAiming`))

(fn `LerpCameraToOrigin`
  (`self.OnPlayerNotAiming`))

(fn `Reload`
  (message `/Game/WeaponSystem/Interface/Input/IInput.Reload` (`self.BP_WeaponController`)))

(fn `SetCanMove`
  (params (NewValue :type Boolean))
  (set `/Game/Blueprint/Player/BP_PlayerController.CanMove` NewValue (`self.PlayerController`)))

(fn `SetSpeed`
  (params (MoveSpeed :type "Float (double-precision)"))
  (set `CharacterMovementComponent.MaxWalkSpeed` MoveSpeed (`self.CharacterMovement`)))

(fn `SetState`
  (params (NewState :type "/Game/Blueprint/Player/E_StateType Enum" :default "NewEnumerator0"))
  (bind (_value _returnvalue) (`BlueprintMapLibrary.Map_Find` (`self.StateMap`) NewState))
  (if _returnvalue
    (bind _output_get (set `self.CurrentState` _value))
    (`/Game/Blueprint/Player/Interfaces/IState.OnEnter` _output_get)
    (`self.OnStateChanged` NewState)
    (else
      (`KismetSystemLibrary.PrintString` "State Not Found" true true (struct :`R` 1.0 :`A` 1.0)))))

(fn `SpecialAttack`)

(fn `UserConstructionScript`)