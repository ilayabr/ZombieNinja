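; Player dash state for a state machine, which applies an impulse to the player through the state machine on entry.
; Entry requires two flags in the state machine's player context map, one false and the other true.
; Tick accumulates time while the state is active, then allows exit and signals that the state has ended once the maximum duration is reached.
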(event `self.ReceiveTick`
  (params (DeltaSeconds :type "Float (single-precision)"))
  (if (`self.StateActive`)
    (bind _output_get (set `self.InStateTimer` (+ DeltaSeconds (`self.InStateTimer`))))
    (if (>= _output_get (`self.MaxTimeInState`))
      (set `self.CanChangeState` true)
      (`self.StateEnded`))))

(event `/Game/Blueprint/Player/Interfaces/IState.OnEnter`
  ; Reset variables
  (set `self.CanChangeState` false)
  (set `self.InStateTimer` 0.0)
  (set `self.StateActive` true)
  (`/Game/Blueprint/Player/BP_PlayerStateMachine.ImpulsePlayer` (`self.StateMachine`) (`self.DashingForce`)))

(event `/Game/Blueprint/Player/Interfaces/IState.OnExit`
  (set `self.StateActive` false))

(fn `CheckEntryCondition`
  (returns (CanEnter :type Boolean))
  (bind _playercontextmap (`/Game/Blueprint/Player/BP_PlayerStateMachine.PlayerContextMap` (`self.StateMachine`)))
  (bind (_value _returnvalue) (`BlueprintMapLibrary.Map_Find` _playercontextmap "NewEnumerator5"))
  (bind (_value_2 _returnvalue_2) (`BlueprintMapLibrary.Map_Find` _playercontextmap "NewEnumerator7"))
  (if _returnvalue
    (if _returnvalue_2
      (return (and (not _value) _value_2))
      (else
        _)))
  (return false))

(fn `CheckExitCondition`
  (returns (CanExit :type Boolean))
  (return (`self.CanChangeState`)))

(fn `UserConstructionScript`)