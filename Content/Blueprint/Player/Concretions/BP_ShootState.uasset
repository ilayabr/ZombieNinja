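; BP_ShootState is the shoot state for the player's state machine.
; It allows entry only when two enum-keyed flags in the state machine's PlayerContextMap both exist and are true.
; Exit is always allowed, and the Blueprint adds no behavior of its own beyond these two condition checks.
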(fn `CheckEntryCondition`
  (returns (CanEnter :type Boolean))
  (bind _playercontextmap (`/Game/Blueprint/Player/BP_PlayerStateMachine.PlayerContextMap` (`self.StateMachine`)))
  (bind (_value _returnvalue) (`BlueprintMapLibrary.Map_Find` _playercontextmap "NewEnumerator4"))
  (bind (_value_2 _returnvalue_2) (`BlueprintMapLibrary.Map_Find` _playercontextmap "NewEnumerator5"))
  (if _returnvalue
    (if _returnvalue_2
      (return (and _value _value_2))
      (else
        _)))
  (return false))

(fn `CheckExitCondition`
  (returns (CanExit :type Boolean))
  (return true))

(fn `UserConstructionScript`)