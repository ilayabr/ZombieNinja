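; Player jump state for a state machine, which launches the player upward with a jump impulse.
; Entry requires the player to be grounded and a flag in the state machine's PlayerContextMap to be true, with a missing entry counting as false.
; On enter it runs the base logic, then passes JumpForce to the state machine's JumpImpulse.
; Exit is allowed whenever CanChangeState is true.
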(event `/Game/Blueprint/Player/Interfaces/IState.OnEnter`
  (`self.BaseOnEnter`)
  (`/Game/Blueprint/Player/BP_PlayerStateMachine.JumpImpulse` (`self.StateMachine`) (`self.JumpForce`)))

(fn `CheckEntryCondition`
  (returns (CanEnter :type Boolean))
  (bind (_value _returnvalue) (`BlueprintMapLibrary.Map_Find` (`/Game/Blueprint/Player/BP_PlayerStateMachine.PlayerContextMap` (`self.StateMachine`)) "NewEnumerator3"))
  (bind _isground (`/Game/Blueprint/Player/BP_PlayerStateMachine.IsGrounded` (`self.StateMachine`)))
  (if _returnvalue
    (if true
      (return (and _value _isground))
      (else
        _)))
  (return false))

(fn `CheckExitCondition`
  (returns (CanExit :type Boolean))
  (return (`self.CanChangeState`)))

(fn `UserConstructionScript`)