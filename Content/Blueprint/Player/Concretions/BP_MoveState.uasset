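; BP_MoveState is the player's move state, defining when a state machine can enter and leave it.
; The entry check reads three boolean flags from the StateMachine's PlayerContextMap by enum key, passing only if all are found, the first is true and the other two are false.
; The exit check always returns true, and the state contains no movement logic of its own.
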(fn `CheckEntryCondition`
  (returns (CanEnter :type Boolean))
  (bind _playercontextmap (`/Game/Blueprint/Player/BP_PlayerStateMachine.PlayerContextMap` (`self.StateMachine`)))
  (bind (_value _returnvalue) (`BlueprintMapLibrary.Map_Find` _playercontextmap "NewEnumerator0"))
  (bind (_value_2 _returnvalue_2) (`BlueprintMapLibrary.Map_Find` _playercontextmap "NewEnumerator5"))
  (bind (_value_3 _returnvalue_3) (`BlueprintMapLibrary.Map_Find` _playercontextmap "NewEnumerator6"))
  (if _returnvalue
    (if _returnvalue_3
      (if _returnvalue_2
        (return (and (and _value (not _value_3)) (not _value_2))))
      (else
        (return false)))
    (else
      (return false))))

(fn `CheckExitCondition`
  (returns (CanExit :type Boolean))
  (return true))

(fn `UserConstructionScript`)