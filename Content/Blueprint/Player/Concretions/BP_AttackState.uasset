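; Player attack state in a state machine, a concrete state that performs the regular sword attack.
; Entry requires the base check plus two flags in the state machine's player context map: one true, the other false.
; On enter it impulses the player forward, triggers a non-special attack through the state machine and plays a delayed swoosh sound.
; Its own exit condition always returns false.
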(event `self.ReceiveBeginPlay`)

(event `self.ReceiveTick`
  (params (DeltaSeconds :type "Float (single-precision)"))
  (`self.BaseTick` DeltaSeconds))

(event `/Game/Blueprint/Player/Interfaces/IState.OnExit`
  (`self.BaseOnExit`))

(event `/Game/Blueprint/Player/Interfaces/IState.OnEnter`
  (bind _statemachine (`self.StateMachine`))
  (`self.BaseOnEnter`)
  (`/Game/Blueprint/Player/BP_PlayerStateMachine.ImpulsePlayerForward` _statemachine (`self.AttackForce`))
  (`/Game/Blueprint/Player/BP_PlayerStateMachine.Attack` _statemachine 50 false)
  (`KismetSystemLibrary.Delay` 0.2)
  (`GameplayStatics.PlaySound2D` "/Game/Effects/Audio/MS_SwordSwoosh.MS_SwordSwoosh" 1.0 1.0 0.0 null null))

(fn `CheckEntryCondition`
  (returns (CanEnter :type Boolean))
  (bind _playercontextmap (`/Game/Blueprint/Player/BP_PlayerStateMachine.PlayerContextMap` (`self.StateMachine`)))
  (bind (_value _returnvalue) (`BlueprintMapLibrary.Map_Find` _playercontextmap "NewEnumerator4"))
  (bind (_value_2 _returnvalue_2) (`BlueprintMapLibrary.Map_Find` _playercontextmap "NewEnumerator5"))
  (bind _canenter (`self.BaseCheckEntryCondition`))
  (if _canenter
    (if _returnvalue
      (if _returnvalue_2
        (return (and _value (not _value_2)))
        (else
          _)))
    (return false)))

(fn `CheckExitCondition`
  (returns (CanExit :type Boolean))
  (return false))

(fn `UserConstructionScript`)