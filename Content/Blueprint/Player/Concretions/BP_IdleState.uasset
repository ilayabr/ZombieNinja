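; BP_IdleState is the idle state for the player's state machine.
; Its entry check passes only when the state machine reports grounded and two PlayerContextMap flags both exist and are false, failing if either key is missing.
; Its exit check always returns true, so the state itself never blocks a transition out.
; The event graph and construction script hold no logic.
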(fn `CheckEntryCondition`
  (returns (CanEnter :type Boolean))
  (bind _statemachine (`self.StateMachine`))
  (bind _playercontextmap (`/Game/Blueprint/Player/BP_PlayerStateMachine.PlayerContextMap` _statemachine))
  (bind (_value _returnvalue) (`BlueprintMapLibrary.Map_Find` _playercontextmap "NewEnumerator5"))
  (bind (_value_2 _returnvalue_2) (`BlueprintMapLibrary.Map_Find` _playercontextmap "NewEnumerator0"))
  (bind _isground (`/Game/Blueprint/Player/BP_PlayerStateMachine.IsGrounded` _statemachine))
  (if _returnvalue_2
    (if _returnvalue
      (return (and (and (not _value_2) (not _value)) _isground))
      (else
        _)))
  (return false))

(fn `CheckExitCondition`
  (returns (CanExit :type Boolean))
  (return true))

(fn `UserConstructionScript`)