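; BP_SpecialAttackState is a player state for the special attack, a forward lunge that deals damage.
; On enter it runs the base logic, impulses the player forward by SpecialAttackForce, then calls the state machine's Attack with a fixed damage and the special flag.
; Entry depends on a flag looked up in the state machine's PlayerContextMap, and exit on CanChangeState.
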(event `/Game/Blueprint/Player/Interfaces/IState.OnEnter`
  (bind _statemachine (`self.StateMachine`))
  (`self.BaseOnEnter`)
  ;[1 1 1] check the forward of the player and dash there check collision with ray or other resourc
  (`/Game/Blueprint/Player/BP_PlayerStateMachine.ImpulsePlayerForward` _statemachine (`self.SpecialAttackForce`))
  (`/Game/Blueprint/Player/BP_PlayerStateMachine.Attack` _statemachine 100 true))

(fn `CheckEntryCondition`
  (returns (CanEnter :type Boolean))
  (bind (_value _returnvalue) (`BlueprintMapLibrary.Map_Find` (`/Game/Blueprint/Player/BP_PlayerStateMachine.PlayerContextMap` (`self.StateMachine`)) "NewEnumerator4"))
  (if _returnvalue
    (return _value)))

(fn `CheckExitCondition`
  (returns (CanExit :type Boolean))
  (return (`self.CanChangeState`)))

(fn `UserConstructionScript`)