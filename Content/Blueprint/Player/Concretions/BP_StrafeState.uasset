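; BP_StrafeState is a player state machine state for strafing, apparently while aiming.
; Entry requires two flags in the state machine's PlayerContextMap to both be present and true, while exit is always allowed.
; On enter it enables movement, sets the speed to StrafeSpeed and fires the state machine's player-aimed event.
; On exit it disables movement and zeroes the speed.
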(event `/Game/Blueprint/Player/Interfaces/IState.OnExit`
  (bind _statemachine (`self.StateMachine`))
  (`/Game/Blueprint/Player/BP_PlayerStateMachine.SetCanMove` _statemachine false)
  (`/Game/Blueprint/Player/BP_PlayerStateMachine.SetSpeed` _statemachine 0.0))

(event `/Game/Blueprint/Player/Interfaces/IState.OnEnter`
  (bind _statemachine (`self.StateMachine`))
  (`/Game/Blueprint/Player/BP_PlayerStateMachine.SetCanMove` _statemachine true)
  (`/Game/Blueprint/Player/BP_PlayerStateMachine.SetSpeed` _statemachine (`self.StrafeSpeed`))
  (`/Game/Blueprint/Player/BP_PlayerStateMachine.OnPlayerAimedEvent` (`self.StateMachine`)))

(fn `CheckEntryCondition`
  (returns (CanEnter :type Boolean))
  (bind _playercontextmap (`/Game/Blueprint/Player/BP_PlayerStateMachine.PlayerContextMap` (`self.StateMachine`)))
  (bind (_value _returnvalue) (`BlueprintMapLibrary.Map_Find` _playercontextmap "NewEnumerator0"))
  (bind (_value_2 _returnvalue_2) (`BlueprintMapLibrary.Map_Find` _playercontextmap "NewEnumerator5"))
  (if _returnvalue
    (if _returnvalue_2
      (return (and _value _value_2)))))

(fn `CheckExitCondition`
  (returns (CanExit :type Boolean))
  (return true))

(fn `UserConstructionScript`)