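; Player state machine state that handles weapon reloading.
; Entry requires a specific player context flag to be set and the weapon controller's reload check to pass.
; On enter it runs the base state logic and then tells the weapon controller to reload.
; Exit is allowed whenever the state's CanChangeState flag is true.
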(event `/Game/Blueprint/Player/Interfaces/IState.OnEnter`
  (`self.BaseOnEnter`)
  (`/Game/WeaponSystem/WeaponContainer/BP_WeaponController.Reload` (`/Game/Blueprint/Player/BP_PlayerStateMachine.WeaponController` (`self.StateMachine`))))

(fn `CheckEntryCondition`
  (returns (CanEnter :type Boolean))
  (bind _statemachine (`self.StateMachine`))
  (bind (_value _returnvalue) (`BlueprintMapLibrary.Map_Find` (`/Game/Blueprint/Player/BP_PlayerStateMachine.PlayerContextMap` _statemachine) "NewEnumerator8"))
  (if _returnvalue
    (bind _canreload (`/Game/WeaponSystem/Interface/Input/IInput.CheckReload` (`/Game/Blueprint/Player/BP_PlayerStateMachine.WeaponController` _statemachine)))
    (return (and _canreload _value))))

(fn `CheckExitCondition`
  (returns (CanExit :type Boolean))
  (return (`self.CanChangeState`)))

(fn `UserConstructionScript`)