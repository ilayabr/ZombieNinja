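; BP_ZombieField runs a timed, round-based zombie survival mode and starts background music on BeginPlay.
; The BP_PlayerDetector overlap event starts the first round, then Tick fires RoundStarted whenever MaxRoundTime elapses, until ZombieAmountArr is exhausted.
; Each round spawns BP_BaseZombie using that round's array count, at random directions within a min/max distance ring around the player, adjusting for or skipping colliding spawns.
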(event `OnRoundStarted` :!signature `self.RoundStarted`
  (params (RoundIndex :type Integer))
  (bind _returnvalue (`self.GetTransform` (`self.PlayerPawn`)))
  (bind (_returnvalue_x _returnvalue_y) (`KismetMathLibrary.BreakVector` (+ (* (`KismetMathLibrary.Vector_Normal2D` (`KismetMathLibrary.MakeVector` (* (`KismetMathLibrary.RandomFloat`) (`self.RandomizePosNeg`)) (* (`KismetMathLibrary.RandomFloat`) (`self.RandomizePosNeg`)))) (`KismetMathLibrary.RandomFloatInRange` (`self.MinimumDistanceFromPlayer`) (`self.MaximumDistanceFromPlayer`))) (`KismetMathLibrary.MakeVector` (.x (.location _returnvalue)) (.y (.location _returnvalue))))))
  ; zombie spawner logic
  (for _index (range (+ (`|GetArrayItem` (`self.ZombieAmountArr`) RoundIndex) 1))
    (`KismetSystemLibrary.PrintString` (`KismetStringLibrary.Conv_IntToString` _index))
    (`|SpawnActorFromClass` "/Game/Blueprint/Enemy/BP_BaseZombie.BP_BaseZombie_C" (`KismetMathLibrary.MakeTransform` (`KismetMathLibrary.MakeVector` _returnvalue_x _returnvalue_y (.z (.location _returnvalue))) (`KismetMathLibrary.MakeRotator` 0.0 (.pitch (.rotation _returnvalue)) (`KismetMathLibrary.RandomFloat`))) "AdjustIfPossibleButDontSpawnIfColliding" "MultiplyWithRoot" null null)))

(event `self.ReceiveBeginPlay`
  (set `self.PlayerPawn` (`GameplayStatics.GetPlayerPawn` 0))
  (add `self.RoundStarted` (delegate `OnRoundStarted`))
  (bind _returnvalue (`GameplayStatics.GetActorOfClass` "/Game/Blueprint/GameMode/BP_PlayerDetector.BP_PlayerDetector_C"))
  (set `self.GameZone` _returnvalue)
  (add `/Game/Blueprint/GameMode/BP_PlayerDetector.PlayerOverlap` _returnvalue (delegate `OnPlayerEnteredZone`))
  (`GameplayStatics.PlaySound2D` "/Game/Effects/Audio/MS_BackgroundMusic.MS_BackgroundMusic" 1.0 1.0 0.0 null null))

(event `OnPlayerEnteredZone`
  ; If Player in zone begin game mode
  (if (not (`self.IsPlayerInZone`))
    (set `self.IsPlayerInZone` true)
    (`self.RoundStarted` 0)))

(event `self.ReceiveTick`
  (params (DeltaSeconds :type "Float (single-precision)"))
  (bind _roundindex (`self.RoundIndex`))
  (if (`self.IsPlayerInZone`)
    (bind _output_get (set `self.Timer` (+ DeltaSeconds (`self.Timer`))))
    (`KismetSystemLibrary.PrintString` (`KismetStringLibrary.Conv_DoubleToString` _output_get) true true (struct :`G` 0.66 :`B` 1.0 :`A` 1.0) 2.0 "timer")
    (if (>= (`self.Timer`) (`self.MaxRoundTime`))
      (set `self.Timer` 0.0)
      (`self.RoundStarted` _roundindex)
      (`/Engine/EditorBlueprintResources/StandardMacros.IncrementInt` _roundindex
        (:`  `
          (if (<= (`KismetArrayLibrary.Array_Length` (`self.ZombieAmountArr`)) (`self.RoundIndex`))
            (set `self.IsPlayerInZone` false)))))))

(fn `RandomizePosNeg`
  (returns (ReturnValue :type Integer))
  (if (== (`KismetMathLibrary.RandomInteger` 2) 1)
    (return 1)
    (else
      (return -1))))

(fn `UserConstructionScript`)