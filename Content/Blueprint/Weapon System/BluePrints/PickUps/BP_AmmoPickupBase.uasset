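; Base Blueprint for ammo pickups in the weapon system, holding an ammo type and amount.
; On BeginPlay it unhides itself, sets a sci-fi mesh and assigns a material for the grenade and medium ammo types.
; GetPickUpData exposes the ammo type, and SetLeftovers overwrites the amount with whatever remains.
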(event `self.ReceiveBeginPlay`
  (bind _staticmesh (`self.StaticMesh`))
  (`self.SetActorHiddenInGame` false)
  (`StaticMeshComponent.SetStaticMesh` (`self.StaticMesh`) "/Game/LP_LiteWeapons_JC/Models/SM_SciFi_Weapons_03.SM_SciFi_Weapons_03")
  (switch `/Game/Enums/E_AmmoType` (`self.AmmoType`)
    (:`NewEnumerator0`
      (`PrimitiveComponent.SetMaterial` _staticmesh 0 "/Engine/VREditor/BasicMeshes/MI_Cube_03.MI_Cube_03"))
    (:`NewEnumerator1`
      (`PrimitiveComponent.SetMaterial` _staticmesh 0 "/Engine/BasicShapes/BasicShapeMaterial.BasicShapeMaterial"))))

(fn `GetPickUpData`
  (returns (PickupType :type "/Game/Enums/E_AmmoType Enum"))
  (return (`self.AmmoType`)))

(fn `SetLeftovers`
  (params (Leftovers :type Integer))
  (set `self.AmmoAmount` Leftovers))

(fn `UserConstructionScript`)